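; 3DPopupWidget is a placeable actor that shows a popup help window in the world while something overlaps its TriggerBox.
; On BeginPlay it casts the widget component's object to PopupHelpWindow, copies in its text, colors and image, and sets initial visibility.
; Overlap begin shows the widget.
; Overlap end hides it, optionally after a timeline opacity fade, and can then destroy the actor for one-time popups.
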(event OnComponentBeginOverlap(TriggerBox)
  (params (OtherActor :type Actor%20Object%20Reference) (OtherComp :type Primitive%20Component%20Object%20Reference) (OtherBodyIndex :type Integer) (bFromSweep :type Boolean) (SweepResult :type Hit%20Result%20Structure%20%28by%20ref%29))
  (Rendering|SetVisibility (Variables|Default|GetWidget) true false))

(event OnComponentEndOverlap(TriggerBox)
  (params (OtherActor :type Actor%20Object%20Reference) (OtherComp :type Primitive%20Component%20Object%20Reference) (OtherBodyIndex :type Integer))
  (if (Variables|Default|GetFadeOut)
    (bind _lerp_1_0 (Timeline|Timeline_0 PlayFromStart)
      (:Update
        (Default|ChangeOpacity (Variables|Default|Get3DTextWidgetRef) _lerp_1_0))
      (:Finished
        (Rendering|SetVisibility (Variables|Default|GetWidget) false false :!label _label)
        (if (Variables|Default|GetDestroyOnEndOverlap)
          (Actor|DestroyActor))))
    (else
      (goto _label))))

(event EventBeginPlay
  (Rendering|SetVisibility (Variables|Default|GetWidget) (Variables|Default|GetStartVisible) false)
  (bind _aspopup_help_window (Utilities|Casting|CastToPopupHelpWindow (UserInterface|GetUserWidgetObject (Variables|Default|GetWidget))))
  (Variables|Default|Set3DTextWidgetRef _aspopup_help_window)
  (Variables|/Game/MyContent/Blueprints/UserInterface/PopupHelpWindow.PopupHelpWindow_C|SetTextToDisplay (Variables|Default|Get3DTextWidgetRef) (Variables|Default|GetTextToDisplay))
  (Variables|/Game/MyContent/Blueprints/UserInterface/PopupHelpWindow.PopupHelpWindow_C|SetBackgroundColor (Variables|Default|Get3DTextWidgetRef) (Variables|Default|GetBackgroundColor))
  (Variables|/Game/MyContent/Blueprints/UserInterface/PopupHelpWindow.PopupHelpWindow_C|SetTextColor (Variables|Default|Get3DTextWidgetRef) (Variables|Default|GetTextColor))
  (Variables|/Game/MyContent/Blueprints/UserInterface/PopupHelpWindow.PopupHelpWindow_C|SetBorderColor (Variables|Default|Get3DTextWidgetRef) (Variables|Default|GetBorderColor))
  (Appearance|SetBrushfromTexture (Variables|/Game/MyContent/Blueprints/UserInterface/PopupHelpWindow.PopupHelpWindow_C|GetKidsImage (Variables|Default|Get3DTextWidgetRef)) (Variables|Default|GetKidsImage) false))

(fn ConstructionScript)
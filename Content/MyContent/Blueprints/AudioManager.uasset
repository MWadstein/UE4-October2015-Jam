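; AudioManager plays random child cry dialogue on the player, picking the voice (Malachi, Michael or Alex) from the character's current Red, Blue or Green area.
; Tick accumulates time and, past the check interval, rolls the cry chance every frame until one passes.
; A passing roll sets full or muted volume from the SaveSlot1 sound setting, then activates reverb, spawns the attached dialogue and resets the timer.
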(event EventTick
  (params (DeltaSeconds :type Float%20%28single-precision%29))
  (Variables|Default|SetTimeSinceLastCheck (+ DeltaSeconds (Variables|Default|GetTimeSinceLastCheck)))
  (Utilities|FlowControl|Sequence
    (:then_0
      ;[1 1 1] Child Cries
      (if (>= (Variables|Default|GetTimeSinceLastCheck) (Variables|Default|GetTimeBetweenSoundChecks))
        (if (<= (Math|Random|RandomFloatinRange 0.0 1.0) (Variables|Cries|GetPercentChanceForCry))
          (CallFunction|SetSoundVolume)
          (bind _asmy_fpcharacter (Utilities|Casting|CastToMyFPCharacter (Game|GetPlayerCharacter 0)))
          (switch Utilities|FlowControl|Switch|SwitchonAreas (Variables|/Game/MyContent/Blueprints/Base/MyFPCharacter.MyFPCharacter_C|GetCurrentArea _asmy_fpcharacter)
            (:NewEnumerator1
              (Class|GameplayStatics|ActivateReverbEffect "/Game/MyContent/Audio/BasicReverb.BasicReverb")
              (Class|GameplayStatics|SpawnDialogueAttached (Utilities|Array|Get(acopy) (Variables|Cries|GetMalachiCries) (Math|Random|RandomIntegerinRange 0 (- (Utilities|Array|Length (Variables|Cries|GetMalachiCries)) 1))) (Variables|Default|GetDC_Malachi) (Variables|/Script/Engine.Character|GetMesh (Game|GetPlayerCharacter 0)) "None" "0, 0, 0" "0, 0, 0" "KeepRelativeOffset" false (Variables|Default|GetVolume))
              (Variables|Default|SetTimeSinceLastCheck 0.0))
            (:NewEnumerator2
              (Class|GameplayStatics|ActivateReverbEffect "/Game/MyContent/Audio/BasicReverb.BasicReverb")
              (Class|GameplayStatics|SpawnDialogueAttached (Utilities|Array|Get(acopy) (Variables|Cries|GetMichaelCries) (Math|Random|RandomIntegerinRange 0 (- (Utilities|Array|Length (Variables|Cries|GetMichaelCries)) 1))) (Variables|Default|GetDC_Michael) (Variables|/Script/Engine.Character|GetMesh (Game|GetPlayerCharacter 0)) "None" "0, 0, 0" "0, 0, 0" "KeepRelativeOffset" false (Variables|Default|GetVolume))
              (Variables|Default|SetTimeSinceLastCheck 0.0))
            (:NewEnumerator3
              (Class|GameplayStatics|ActivateReverbEffect "/Game/MyContent/Audio/BasicReverb.BasicReverb")
              (Class|GameplayStatics|SpawnDialogueAttached (Utilities|Array|Get(acopy) (Variables|Cries|GetAlexCries) (Math|Random|RandomIntegerinRange 0 (- (Utilities|Array|Length (Variables|Cries|GetAlexCries)) 1))) (Variables|Default|GetDC_Alex) (Variables|/Script/Engine.Character|GetMesh (Game|GetPlayerCharacter 0)) "None" "0, 0, 0" "0, 0, 0" "KeepRelativeOffset" false (Variables|Default|GetVolume))
              (Variables|Default|SetTimeSinceLastCheck 0.0))))))))

(fn ConstructionScript)

(fn SetSoundVolume
  (bind _returnvalue (SaveGame|LoadGamefromSlot "SaveSlot1"))
  (bind _asmy_save_game (Utilities|Casting|CastToMySaveGame _returnvalue))
  (if (Variables|/Game/MyContent/Blueprints/Base/MySaveGame.MySaveGame_C|GetSounds _asmy_save_game)
    (Variables|Default|SetVolume 1.0)
    (else
      (Variables|Default|SetVolume 0.0))))
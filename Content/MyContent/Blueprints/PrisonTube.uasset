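; Prison tube actor that, on LowerTube, sinks from its starting position and is then sealed off by its separate CoverPlatform.
; LowerTube destroys the IdWidget actor, then runs two chained timelines that lerp the tube down and then raise the cover.
; An attached hum plays during the motion and gives way to a double thud at the end, with volume muted or full per the Sounds flag in the save game.
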(event Custom|LowerTube
  (bind _coverstartingposition (Variables|Default|GetCoverStartingPosition))
  (bind _coverstartingposition_2 (Variables|Default|GetCoverStartingPosition))
  (bind _prisonstartingposition (Variables|Default|GetPrisonStartingPosition))
  (bind _prisonstartingposition_2 (Variables|Default|GetPrisonStartingPosition))
  (Actor|DestroyActor (Variables|Default|GetIdWidget))
  (bind _returnvalue (SaveGame|LoadGamefromSlot "SaveSlot1"))
  (bind _asmy_save_game (Utilities|Casting|CastToMySaveGame _returnvalue))
  (if (Variables|/Game/MyContent/Blueprints/Base/MySaveGame.MySaveGame_C|GetSounds _asmy_save_game)
    (Variables|Default|SetSoundVolume 1.0)
    (else
      (Variables|Default|SetSoundVolume 0.0)))
  (bind _returnvalue_2 (Audio|SpawnSoundAttached "/Game/MyContent/Audio/Effects/fx-hum.fx-hum" (Variables|Default|GetRoot) "None" (Transformation|GetWorldLocation (Variables|Default|GetRoot)) "0, 0, 0" "KeepRelativeOffset" false (Variables|Default|GetSoundVolume)))
  (Variables|Default|SetHumSound _returnvalue_2)
  (bind _lerp (Timeline|Timeline_0 PlayFromStart)
    (:Update
      (Transformation|SetWorldLocation (Variables|Default|GetRoot) (Math|Vector|Lerp(Vector) (Math|Vector|MakeVector (.x _prisonstartingposition) (.y _prisonstartingposition) (.z _prisonstartingposition)) (Math|Vector|MakeVector (.x _prisonstartingposition_2) (.y _prisonstartingposition_2) (- (.z _prisonstartingposition_2) 5.5e+02)) _lerp) false false))
    (:Finished
      (bind _lerp_2 (Timeline|Timeline_1 Play)
        (:Update
          (Transformation|SetWorldLocation (Variables|/Game/MyContent/Blueprints/Platforms/Platform.Platform_C|GetRoot (Variables|Default|GetCoverPlatform)) (Math|Vector|Lerp(Vector) (Math|Vector|MakeVector (.x _coverstartingposition_2) (.y _coverstartingposition_2) (.z _coverstartingposition_2)) (Math|Vector|MakeVector (.x _coverstartingposition) (.y _coverstartingposition) (+ (.z _coverstartingposition) 5e+01)) _lerp_2) false false))
        (:Finished
          (Audio|Components|Audio|Stop (Variables|Default|GetHumSound))
          (Audio|PlaySoundatLocation "/Game/MyContent/Audio/Effects/fx-DoubleThud.fx-DoubleThud" (Transformation|GetWorldLocation (Variables|Default|GetRoot)) "0, 0, 0" (Variables|Default|GetSoundVolume)))))))

(event EventBeginPlay
  (Variables|Default|SetPrisonStartingPosition (Transformation|GetWorldLocation (Variables|Default|GetRoot)))
  (Variables|Default|SetCoverStartingPosition (Transformation|GetWorldLocation (Variables|/Game/MyContent/Blueprints/Platforms/Platform.Platform_C|GetRoot (Variables|Default|GetCoverPlatform)))))

(fn ConstructionScript)
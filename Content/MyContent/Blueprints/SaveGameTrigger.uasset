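; SaveGameTrigger is a trigger volume that writes a save game when anything begins overlapping its Box component.
; Each overlap creates a new MySaveGame object and sets its CurrentMap to the trigger's MapName, then saves it to a fixed slot.
; SavedBlue, SavedGreen and SavedRed are assigned from the new object itself, so they keep class defaults rather than earlier saved values.
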(event OnComponentBeginOverlap(Box)
  (params (OtherActor :type Actor%20Object%20Reference) (OtherComp :type Primitive%20Component%20Object%20Reference) (OtherBodyIndex :type Integer) (bFromSweep :type Boolean) (SweepResult :type Hit%20Result%20Structure%20%28by%20ref%29))
  (bind _returnvalue (SaveGame|CreateSaveGameObject "/Game/MyContent/Blueprints/MySaveGame.MySaveGame_C"))
  (bind _asmy_save_game (Utilities|Casting|CastToMySaveGame _returnvalue))
  (bind _output_get (Variables|Default|SetSaveInstance _asmy_save_game))
  (Variables|/Game/MyContent/Blueprints/MySaveGame.MySaveGame_C|SetCurrentMap _output_get (Variables|Default|GetMapName))
  (Variables|/Game/MyContent/Blueprints/MySaveGame.MySaveGame_C|SetSavedBlue (Variables|Default|GetSaveInstance) (Variables|/Game/MyContent/Blueprints/MySaveGame.MySaveGame_C|GetSavedBlue (Variables|Default|GetSaveInstance)))
  (Variables|/Game/MyContent/Blueprints/MySaveGame.MySaveGame_C|SetSavedGreen (Variables|Default|GetSaveInstance) (Variables|/Game/MyContent/Blueprints/MySaveGame.MySaveGame_C|GetSavedGreen (Variables|Default|GetSaveInstance)))
  (Variables|/Game/MyContent/Blueprints/MySaveGame.MySaveGame_C|SetSavedRed (Variables|Default|GetSaveInstance) (Variables|/Game/MyContent/Blueprints/MySaveGame.MySaveGame_C|GetSavedRed (Variables|Default|GetSaveInstance)))
  (SaveGame|SaveGametoSlot (Variables|Default|GetSaveInstance) "SaveSlot1"))

(fn ConstructionScript)
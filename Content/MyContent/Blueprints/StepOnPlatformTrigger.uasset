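; A trigger actor that plays a one-time "step on platform" voiceover when a player enters its box.
; On overlap by an actor implementing the Player interface, it loads the save game and checks whether the voiceover is still pending.
; It plays the dialogue wave at its own location, zeroing the volume if the saved sound setting is off.
; It then clears the saved flag and writes the slot, so the line does not repeat.
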(event OnComponentBeginOverlap(Box)
  (params (OtherActor :type Actor%20Object%20Reference) (OtherComp :type Primitive%20Component%20Object%20Reference) (OtherBodyIndex :type Integer) (bFromSweep :type Boolean) (SweepResult :type Hit%20Result%20Structure%20%28by%20ref%29))
  (if (Utilities|DoesObjectImplementInterface OtherActor "/Game/MyContent/Blueprints/Interfaces/Player.Player_C")
    (bind _returnvalue (SaveGame|LoadGamefromSlot "SaveSlot1"))
    (bind _asmy_save_game (Utilities|Casting|CastToMySaveGame _returnvalue))
    (bind _output_get (Variables|Default|SetSaveInstance _asmy_save_game))
    (if (Variables|/Game/MyContent/Blueprints/Base/MySaveGame.MySaveGame_C|GetPlayPlatformVoiceover _output_get)
      (if (Variables|/Game/MyContent/Blueprints/Base/MySaveGame.MySaveGame_C|GetSounds _output_get)
        _
        (else
          (Variables|Default|SetVolume 0.0)))
      (Class|GameplayStatics|PlayDialogueatLocation "/Game/MyContent/Audio/Mathew/DW_mathew-StepOnPlatform.DW_mathew-StepOnPlatform" (Variables|Default|GetDC_Mathew) (Transformation|GetWorldLocation (Variables|Default|GetRoot)) "0, 0, 0" (Variables|Default|GetVolume))
      (Variables|/Game/MyContent/Blueprints/Base/MySaveGame.MySaveGame_C|SetPlayPlatformVoiceover (Variables|Default|GetSaveInstance) false)
      (SaveGame|SaveGametoSlot (Variables|Default|GetSaveInstance) "SaveSlot1"))))

(fn ConstructionScript)
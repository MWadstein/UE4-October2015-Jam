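; Main room trigger volume that sets the blue, red and green blockers from saved progress and hosts the game-over sequence.
; On player overlap it reads SaveSlot1, toggles the blockers and plays the Mathew/Michelle intro dialogue while its save flag is set, restricting movement.
; HandleGameOverSequence plays ending dialogue, lowers PrisonTubes, fades to black, resets the save except sound and subtitle settings, then loads MainMenu and respawns the player.
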(event OnComponentBeginOverlap(Box)
  (params (OtherActor :type Actor%20Object%20Reference) (OtherComp :type Primitive%20Component%20Object%20Reference) (OtherBodyIndex :type Integer) (bFromSweep :type Boolean) (SweepResult :type Hit%20Result%20Structure%20%28by%20ref%29))
  (if (Utilities|DoesObjectImplementInterface OtherActor "/Game/MyContent/Blueprints/Interfaces/Player.Player_C")
    (bind _returnvalue (SaveGame|LoadGamefromSlot "SaveSlot1"))
    (bind _asmy_save_game (Utilities|Casting|CastToMySaveGame _returnvalue))
    (Variables|Default|SetSaveInstance _asmy_save_game)
    (Utilities|FlowControl|Sequence
      (:then_0
        (Default|ToggleBlocker (Variables|Default|GetBlueBlocker) (Variables|/Game/MyContent/Blueprints/Base/MySaveGame.MySaveGame_C|GetSavedBlue (Variables|Default|GetSaveInstance))))
      (:then_1
        (Default|ToggleBlocker (Variables|Default|GetRedBlocker) (Variables|/Game/MyContent/Blueprints/Base/MySaveGame.MySaveGame_C|GetSavedRed (Variables|Default|GetSaveInstance))))
      (:then_2
        (Default|ToggleBlocker (Variables|Default|GetGreenBlocker) (Variables|/Game/MyContent/Blueprints/Base/MySaveGame.MySaveGame_C|GetSavedGreen (Variables|Default|GetSaveInstance)))))
    (if (Variables|/Game/MyContent/Blueprints/Base/MySaveGame.MySaveGame_C|GetPlayMainRoomIntro (Variables|Default|GetSaveInstance)) ; play main room intro?
      (Utilities|FlowControl|Delay 2.0)
      (Variables|Default|SetSoundLoc (Transformation|GetWorldLocation (Variables|Default|GetDefaultSceneRoot)))
      (bind _asmy_fpcharacter (Utilities|Casting|CastToMyFPCharacter (Game|GetPlayerCharacter 0)))
      (Default|TakeInputfromPlayer _asmy_fpcharacter true false)
      (bind _returnvalue_2 (SaveGame|LoadGamefromSlot "SaveSlot1"))
      (bind _asmy_save_game_2 (Utilities|Casting|CastToMySaveGame _returnvalue_2))
      (if (Variables|/Game/MyContent/Blueprints/Base/MySaveGame.MySaveGame_C|GetSounds _asmy_save_game_2)
        _
        (else
          (Variables|Default|SetVolume 0.0)))
      (Class|GameplayStatics|PlayDialogueatLocation "/Game/MyContent/Audio/Mathew/DW_mathew-MichelleEcho.DW_mathew-MichelleEcho" (Variables|Default|GetDC_Mathew) (Variables|Default|GetSoundLoc) "0, 0, 0" (Variables|Default|GetVolume))
      (Utilities|FlowControl|Delay 1.8)
      (Class|GameplayStatics|PlayDialogueatLocation "/Game/MyContent/Audio/Michelle/DW_michelle-Matt.DW_michelle-Matt" (Variables|Default|GetDC_Michelle) (Variables|Default|GetSoundLoc) "0, 0, 0" (Variables|Default|GetVolume))
      (Utilities|FlowControl|Delay 1.0)
      (Class|GameplayStatics|PlayDialogueatLocation "/Game/MyContent/Audio/Mathew/DW_mathew-CanYouHearMe.DW_mathew-CanYouHearMe" (Variables|Default|GetDC_Mathew) (Variables|Default|GetSoundLoc) "0, 0, 0" (Variables|Default|GetVolume))
      (Utilities|FlowControl|Delay 1.8)
      (Class|GameplayStatics|PlayDialogueatLocation "/Game/MyContent/Audio/Michelle/DW_michelle-MattWhatIsGoing.DW_michelle-MattWhatIsGoing" (Variables|Default|GetDC_Michelle) (Variables|Default|GetSoundLoc) "0, 0, 0" (Variables|Default|GetVolume))
      (Utilities|FlowControl|Delay 2.0)
      (Class|GameplayStatics|PlayDialogueatLocation "/Game/MyContent/Audio/Mathew/DW_mathew-IBrokeIn.DW_mathew-IBrokeIn" (Variables|Default|GetDC_Mathew) (Variables|Default|GetSoundLoc) "0, 0, 0" (Variables|Default|GetVolume))
      (Utilities|FlowControl|Delay 5.0)
      (Class|GameplayStatics|PlayDialogueatLocation "/Game/MyContent/Audio/Mathew/DW_mathew-TookOurKids.DW_mathew-TookOurKids" (Variables|Default|GetDC_Mathew) (Variables|Default|GetSoundLoc) "0, 0, 0" (Variables|Default|GetVolume))
      (Utilities|FlowControl|Delay 2.5)
      (Class|GameplayStatics|PlayDialogueatLocation "/Game/MyContent/Audio/Mathew/DW_mathew-ThePutUsIn.DW_mathew-ThePutUsIn" (Variables|Default|GetDC_Mathew) (Variables|Default|GetSoundLoc) "0, 0, 0" (Variables|Default|GetVolume))
      (Utilities|FlowControl|Delay 6.5)
      (Class|GameplayStatics|PlayDialogueatLocation "/Game/MyContent/Audio/Michelle/DW_michelle-WhyIsThisHappening.DW_michelle-WhyIsThisHappening" (Variables|Default|GetDC_Michelle) (Variables|Default|GetSoundLoc) "0, 0, 0" (Variables|Default|GetVolume))
      (Utilities|FlowControl|Delay 3.2)
      (Class|GameplayStatics|PlayDialogueatLocation "/Game/MyContent/Audio/Mathew/DW_mathew-IWillHelp.DW_mathew-IWillHelp" (Variables|Default|GetDC_Mathew) (Variables|Default|GetSoundLoc) "0, 0, 0" (Variables|Default|GetVolume))
      (Utilities|FlowControl|Delay 5.0)
      (Variables|/Game/MyContent/Blueprints/Base/MySaveGame.MySaveGame_C|SetPlayMainRoomIntro (Variables|Default|GetSaveInstance) false)
      (SaveGame|SaveGametoSlot (Variables|Default|GetSaveInstance) "SaveSlot1")
      (bind _asmy_fpcharacter_2 (Utilities|Casting|CastToMyFPCharacter (Game|GetPlayerCharacter 0)))
      (Default|GiveInputtoPlayer _asmy_fpcharacter_2 true true))))

(event Custom|CheckForBlockers
  (if (Utilities|DoesObjectImplementInterface (stale OnComponentBeginOverlap(Box) OtherActor) "/Game/MyContent/Blueprints/Interfaces/Player.Player_C")
    (bind _returnvalue (SaveGame|LoadGamefromSlot "SaveSlot1"))
    (bind _asmy_save_game (Utilities|Casting|CastToMySaveGame _returnvalue))
    (Variables|Default|SetSaveInstance _asmy_save_game)
    (Utilities|FlowControl|Sequence
      (:then_0
        (Default|ToggleBlocker (Variables|Default|GetBlueBlocker) (Variables|/Game/MyContent/Blueprints/Base/MySaveGame.MySaveGame_C|GetSavedBlue (Variables|Default|GetSaveInstance))))
      (:then_1
        (Default|ToggleBlocker (Variables|Default|GetRedBlocker) (Variables|/Game/MyContent/Blueprints/Base/MySaveGame.MySaveGame_C|GetSavedRed (Variables|Default|GetSaveInstance))))
      (:then_2
        (Default|ToggleBlocker (Variables|Default|GetGreenBlocker) (Variables|/Game/MyContent/Blueprints/Base/MySaveGame.MySaveGame_C|GetSavedGreen (Variables|Default|GetSaveInstance)))))
    (if (Variables|/Game/MyContent/Blueprints/Base/MySaveGame.MySaveGame_C|GetPlayMainRoomIntro (Variables|Default|GetSaveInstance)) ; play main room intro?
      (Utilities|FlowControl|Delay 2.0)
      (Variables|Default|SetSoundLoc (Transformation|GetWorldLocation (Variables|Default|GetDefaultSceneRoot)))
      (bind _asmy_fpcharacter (Utilities|Casting|CastToMyFPCharacter (Game|GetPlayerCharacter 0)))
      (Default|TakeInputfromPlayer _asmy_fpcharacter true false)
      (bind _returnvalue_2 (SaveGame|LoadGamefromSlot "SaveSlot1"))
      (bind _asmy_save_game_2 (Utilities|Casting|CastToMySaveGame _returnvalue_2))
      (if (Variables|/Game/MyContent/Blueprints/Base/MySaveGame.MySaveGame_C|GetSounds _asmy_save_game_2)
        _
        (else
          (Variables|Default|SetVolume 0.0)))
      (Class|GameplayStatics|PlayDialogueatLocation "/Game/MyContent/Audio/Mathew/DW_mathew-MichelleEcho.DW_mathew-MichelleEcho" (Variables|Default|GetDC_Mathew) (Variables|Default|GetSoundLoc) "0, 0, 0" (Variables|Default|GetVolume))
      (Utilities|FlowControl|Delay 1.8)
      (Class|GameplayStatics|PlayDialogueatLocation "/Game/MyContent/Audio/Michelle/DW_michelle-Matt.DW_michelle-Matt" (Variables|Default|GetDC_Michelle) (Variables|Default|GetSoundLoc) "0, 0, 0" (Variables|Default|GetVolume))
      (Utilities|FlowControl|Delay 1.0)
      (Class|GameplayStatics|PlayDialogueatLocation "/Game/MyContent/Audio/Mathew/DW_mathew-CanYouHearMe.DW_mathew-CanYouHearMe" (Variables|Default|GetDC_Mathew) (Variables|Default|GetSoundLoc) "0, 0, 0" (Variables|Default|GetVolume))
      (Utilities|FlowControl|Delay 1.8)
      (Class|GameplayStatics|PlayDialogueatLocation "/Game/MyContent/Audio/Michelle/DW_michelle-MattWhatIsGoing.DW_michelle-MattWhatIsGoing" (Variables|Default|GetDC_Michelle) (Variables|Default|GetSoundLoc) "0, 0, 0" (Variables|Default|GetVolume))
      (Utilities|FlowControl|Delay 2.0)
      (Class|GameplayStatics|PlayDialogueatLocation "/Game/MyContent/Audio/Mathew/DW_mathew-IBrokeIn.DW_mathew-IBrokeIn" (Variables|Default|GetDC_Mathew) (Variables|Default|GetSoundLoc) "0, 0, 0" (Variables|Default|GetVolume))
      (Utilities|FlowControl|Delay 5.0)
      (Class|GameplayStatics|PlayDialogueatLocation "/Game/MyContent/Audio/Mathew/DW_mathew-TookOurKids.DW_mathew-TookOurKids" (Variables|Default|GetDC_Mathew) (Variables|Default|GetSoundLoc) "0, 0, 0" (Variables|Default|GetVolume))
      (Utilities|FlowControl|Delay 2.5)
      (Class|GameplayStatics|PlayDialogueatLocation "/Game/MyContent/Audio/Mathew/DW_mathew-ThePutUsIn.DW_mathew-ThePutUsIn" (Variables|Default|GetDC_Mathew) (Variables|Default|GetSoundLoc) "0, 0, 0" (Variables|Default|GetVolume))
      (Utilities|FlowControl|Delay 6.5)
      (Class|GameplayStatics|PlayDialogueatLocation "/Game/MyContent/Audio/Michelle/DW_michelle-WhyIsThisHappening.DW_michelle-WhyIsThisHappening" (Variables|Default|GetDC_Michelle) (Variables|Default|GetSoundLoc) "0, 0, 0" (Variables|Default|GetVolume))
      (Utilities|FlowControl|Delay 3.2)
      (Class|GameplayStatics|PlayDialogueatLocation "/Game/MyContent/Audio/Mathew/DW_mathew-IWillHelp.DW_mathew-IWillHelp" (Variables|Default|GetDC_Mathew) (Variables|Default|GetSoundLoc) "0, 0, 0" (Variables|Default|GetVolume))
      (Utilities|FlowControl|Delay 5.0)
      (Variables|/Game/MyContent/Blueprints/Base/MySaveGame.MySaveGame_C|SetPlayMainRoomIntro (Variables|Default|GetSaveInstance) false)
      (SaveGame|SaveGametoSlot (Variables|Default|GetSaveInstance) "SaveSlot1")
      (bind _asmy_fpcharacter_2 (Utilities|Casting|CastToMyFPCharacter (Game|GetPlayerCharacter 0)))
      (Default|GiveInputtoPlayer _asmy_fpcharacter_2 true true))))

(event Custom|HandleGameOverSequence
  (CallFunction|HandleDialogforGameOver)
  (bind _asmy_fpcharacter (Utilities|Casting|CastToMyFPCharacter (Game|GetPlayerCharacter 0)))
  (Variables|/Game/MyContent/Blueprints/Base/MyFPCharacter.MyFPCharacter_C|SetGameStarted _asmy_fpcharacter false)
  (Utilities|FlowControl|Delay 2.0)
  (bind _outactors (Actor|GetAllActorsOfClass "/Game/MyContent/Blueprints/PrisonTube.PrisonTube_C"))
  (for _array_element _outactors
    (Default|LowerTube _array_element))
  (Utilities|FlowControl|Delay 25.0)
  (bind _asmy_fpcharacter_2 (Utilities|Casting|CastToMyFPCharacter (Game|GetPlayerCharacter 0)))
  (Default|TakeInputfromPlayer _asmy_fpcharacter_2 true true)
  (Variables|/Game/MyContent/Blueprints/UserInterface/GameUI.GameUI_C|SetShouldFadeBlackIn (Variables|/Game/MyContent/Blueprints/Base/MyFPCharacter.MyFPCharacter_C|GetUI_Ref _asmy_fpcharacter_2) true)
  (Utilities|FlowControl|Delay 5.0)
  (CallFunction|ClearSaveGame)
  (CallFunction|RemoveSpawnPoint)
  (Game|LoadStreamLevel(byName) "MainMenu" true true)
  (bind _asmy_fpcharacter_3 (Utilities|Casting|CastToMyFPCharacter (Game|GetPlayerCharacter 0)))
  (Default|RespawnatSpawnPoint _asmy_fpcharacter_3 true)
  (Class|Image|SetOpacity (Variables|/Game/MyContent/Blueprints/UserInterface/GameUI.GameUI_C|GetBlackoutImage (Variables|/Game/MyContent/Blueprints/Base/MyFPCharacter.MyFPCharacter_C|GetUI_Ref _asmy_fpcharacter_2)) 0.0))

(event Custom|HandleDialogForGameOver
  (bind _returnvalue (Game|GetPlayerCharacter 0))
  (bind _mesh (Variables|/Script/Engine.Character|GetMesh _returnvalue))
  (bind _returnvalue_2 (Transformation|GetWorldLocation _mesh))
  (bind _returnvalue_3 (SaveGame|LoadGamefromSlot "SaveSlot1"))
  (bind _asmy_save_game (Utilities|Casting|CastToMySaveGame _returnvalue_3))
  (if (Variables|/Game/MyContent/Blueprints/Base/MySaveGame.MySaveGame_C|GetSounds _asmy_save_game)
    (Variables|Default|SetVolume 1.0)
    (else
      (Variables|Default|SetVolume 0.0)))
  (bind _asmy_fpcharacter (Utilities|Casting|CastToMyFPCharacter _returnvalue))
  (Variables|/Game/MyContent/Blueprints/Base/MyFPCharacter.MyFPCharacter_C|SetGameStarted _asmy_fpcharacter false)
  (Class|GameplayStatics|PlayDialogueatLocation "/Game/MyContent/Audio/Mathew/DW_mathew-end1.DW_mathew-end1" (Variables|Default|GetDC_Mathew) _returnvalue_2 "0, 0, 0" (Variables|Default|GetVolume))
  (Utilities|FlowControl|Delay 8.0)
  (Class|GameplayStatics|PlayDialogueatLocation "/Game/MyContent/Audio/Michelle/DW_michelle-End1.DW_michelle-End1" (Variables|Default|GetDC_Michelle) _returnvalue_2 "0, 0, 0" (Variables|Default|GetVolume))
  (Utilities|FlowControl|Delay 5.8)
  (Class|GameplayStatics|PlayDialogueatLocation "/Game/MyContent/Audio/Mathew/DW_mathew-end2.DW_mathew-end2" (Variables|Default|GetDC_Mathew) _returnvalue_2 "0, 0, 0" (Variables|Default|GetVolume))
  (Utilities|FlowControl|Delay 8.0)
  (Class|GameplayStatics|PlayDialogueatLocation "/Game/MyContent/Audio/Michelle/DW_michelle-End2.DW_michelle-End2" (Variables|Default|GetDC_Michelle) _returnvalue_2 "0, 0, 0" (Variables|Default|GetVolume)))

(fn ConstructionScript)

(fn RemoveSpawnPoint
  (bind _outactors (Actor|GetAllActorsOfClass "/Game/MyContent/Blueprints/RespawnPoint.RespawnPoint_C"))
  (Actor|DestroyActor (Utilities|Array|Get(acopy) _outactors)))

(fn ClearSaveGame
  (bind _returnvalue (SaveGame|LoadGamefromSlot "SaveSlot1"))
  (bind _asmy_save_game (Utilities|Casting|CastToMySaveGame _returnvalue))
  (bind _returnvalue_2 (SaveGame|CreateSaveGameObject "/Game/MyContent/Blueprints/Base/MySaveGame.MySaveGame_C"))
  (bind _asmy_save_game_2 (Utilities|Casting|CastToMySaveGame _returnvalue_2))
  (Variables|/Game/MyContent/Blueprints/Base/MySaveGame.MySaveGame_C|SetSounds _asmy_save_game_2 (Variables|/Game/MyContent/Blueprints/Base/MySaveGame.MySaveGame_C|GetSounds _asmy_save_game))
  (Variables|/Game/MyContent/Blueprints/Base/MySaveGame.MySaveGame_C|SetSubtitles _asmy_save_game_2 (Variables|/Game/MyContent/Blueprints/Base/MySaveGame.MySaveGame_C|GetSubtitles _asmy_save_game))
  (SaveGame|SaveGametoSlot _asmy_save_game_2 "SaveSlot1"))
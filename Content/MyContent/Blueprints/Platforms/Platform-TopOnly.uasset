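; Top-only platform Blueprint that acts as one step in a linked chain of platforms, reacting when its Collider is overlapped.
; The overlap swaps the mesh to a landed material, then sets collision, toggles the hint material and updates hiding on each next platform.
; It also tells each previous platform it is done and marks itself visible.
; BeginPlay and construction only call the parent class.
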(event OnComponentBeginOverlap(Collider)
  (params (OtherActor :type Actor%20Object%20Reference) (OtherComp :type Primitive%20Component%20Object%20Reference) (OtherBodyIndex :type Integer) (bFromSweep :type Boolean) (SweepResult :type Hit%20Result%20Structure%20%28by%20ref%29))
  (Rendering|Material|SetMaterial (Variables|Character|GetMesh) 0 (Variables|Default|GetLandedMaterial))
  (Utilities|FlowControl|Sequence
    (:then_0
      (if (> (Utilities|Array|Length (Variables|Default|GetNextPlatforms)) 0)
        (for _array_element (Variables|Default|GetNextPlatforms)
          (Default|ToggleCollision _array_element (Variables|Default|GetNextCollision))
          (Default|ToggleHintMaterial _array_element)
          (Default|ToggleHide _array_element false))))
    (:then_1
      (if (> (Utilities|Array|Length (Variables|Default|GetPreviousPlatforms)) 0)
        (for _array_element_2 (Variables|Default|GetPreviousPlatforms)
          (Default|DonewithPlatform _array_element_2))))
    (:then_2
      (Variables|Default|SetIsVisible true))))

(event EventBeginPlay
  (|CallParentFunction))

(fn ConstructionScript
  (|CallParentFunction))
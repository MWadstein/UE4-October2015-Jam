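; Platform actor that switches between starting, hint and done states by changing its mesh material, collision and visibility.
; BeginPlay resets it to its starting state, and DoneWithPlatform applies the done settings once until the next reset.
; ToggleHide runs last in both, so its collision setting overrides the configured start and done collision.
; Sequence and story-mode events are empty stubs.
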(event Custom|ToggleCollision
  (params (CollisionType :type ECollisionEnabled%20Enum))
  (Collision|SetCollisionEnabled (Variables|Default|GetMesh) CollisionType)
  (Collision|SetCollisionEnabled (Variables|Default|GetCollider) CollisionType))

(event Custom|ToggleHintMaterial
  (Rendering|Material|SetMaterial (Variables|Default|GetMesh) 0 (Variables|Setup|GetHintMaterial)))

(event Custom|ResetPlatform
  (Rendering|Material|SetMaterial (Variables|Default|GetMesh) 0 (Variables|Setup|GetStartingMaterial))
  (Collision|SetCollisionEnabled (Variables|Default|GetMesh) (Variables|Setup|GetStartingCollision))
  (Collision|SetCollisionEnabled (Variables|Default|GetCollider) (Variables|Setup|GetStartingCollision))
  (CallFunction|ToggleHide (Variables|Setup|GetHideAtStart))
  (Variables|Default|SetChangeMaterials true)
  (Variables|Default|SetIsVisible (not (Variables|Setup|GetHideAtStart))))

(event Custom|StartSequence)

(event Custom|GetStoryMode)

(event Custom|DoneWithPlatform
  (if (Variables|Default|GetChangeMaterials)
    (Rendering|Material|SetMaterial (Variables|Default|GetMesh) 0 (Variables|Setup|GetDoneMaterial))
    (Variables|Default|SetChangeMaterials false)
    (Collision|SetCollisionEnabled (Variables|Default|GetMesh) (Variables|Setup|GetCollsionWhenDone))
    (Collision|SetCollisionEnabled (Variables|Default|GetCollider) (Variables|Setup|GetCollsionWhenDone))
    (CallFunction|ToggleHide (Variables|Setup|GetHideWhenDone))))

(event Custom|EndSequence)

(event EventBeginPlay
  (Rendering|Material|CreateDynamicMaterialInstance (Variables|Default|GetMesh) 0 (Variables|Setup|GetStartingMaterial) :!class /Script/Engine.PrimitiveComponent)
  (CallFunction|ResetPlatform))

(fn ConstructionScript)

(fn ToggleHide
  (params (Hidden :type Boolean))
  (if Hidden
    (Collision|SetCollisionEnabled (Variables|Default|GetMesh) "NoCollision")
    (Collision|SetCollisionEnabled (Variables|Default|GetCollider) "NoCollision")
    (Rendering|SetVisibility (Variables|Default|GetMesh) false false)
    (else
      (Collision|SetCollisionEnabled (Variables|Default|GetMesh) "QueryAndPhysics")
      (Collision|SetCollisionEnabled (Variables|Default|GetCollider) "QueryAndPhysics")
      (Rendering|SetVisibility (Variables|Default|GetMesh) true false))))
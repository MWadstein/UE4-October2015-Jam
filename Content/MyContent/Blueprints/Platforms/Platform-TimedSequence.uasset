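; Timed platform that links with others into a chain of appearing and disappearing steps, triggered once when the player overlaps a start platform.
; Starting a platform unhides it with a hint material, tells its previous platforms to end, then starts its next platforms after a delay.
; Ending switches to a done material and hides the platform after a delay, adjusted when the save game has Story Mode enabled.
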(event OnComponentBeginOverlap(Collider)
  (params (OtherActor :type Actor%20Object%20Reference) (OtherComp :type Primitive%20Component%20Object%20Reference) (OtherBodyIndex :type Integer) (bFromSweep :type Boolean) (SweepResult :type Hit%20Result%20Structure%20%28by%20ref%29))
  (if (Math|Boolean|ANDBoolean (Utilities|DoesObjectImplementInterface OtherActor "/Game/MyContent/Blueprints/Interfaces/Player.Player_C") (Variables|Sequence|GetIsStartPlatform) (not (Variables|Default|GetSequenceStarted)))
    (CallFunction|StartSequence)
    (Variables|Default|SetSequenceStarted true)))

(event EventBeginPlay
  (|CallParentFunction)
  (bind _returnvalue (SaveGame|LoadGamefromSlot "SaveSlot1"))
  (bind _asmy_save_game (Utilities|Casting|CastToMySaveGame _returnvalue))
  (if (Variables|/Game/MyContent/Blueprints/Base/MySaveGame.MySaveGame_C|GetStoryMode _asmy_save_game)
    (Variables|Default|SetStoryModeValue (Variables|Default|GetStoryModeAdjust))))

(event EventStartSequence
  (Utilities|FlowControl|Sequence
    (:then_0
      (CallFunction|ToggleHide false))
    (:then_1
      (Rendering|Material|SetMaterial (Variables|Character|GetMesh) 0 (Variables|Default|GetHintMaterial))
      (if (> (Utilities|Array|Length (Variables|Default|GetPreviousPlatforms)) 0)
        (for _array_element (Variables|Default|GetPreviousPlatforms)
          (Default|EndSequence _array_element))))
    (:then_2
      (Utilities|FlowControl|Delay (Variables|Sequence|GetDelayNextStart))
      (if (> (Utilities|Array|Length (Variables|Default|GetNextPlatforms)) 0)
        (for _array_element_2 (Variables|Default|GetNextPlatforms)
          (Default|StartSequence _array_element_2))))))

(event EventEndSequence
  (Rendering|Material|SetMaterial (Variables|Character|GetMesh) 0 (Variables|Default|GetDoneMaterial))
  (Utilities|FlowControl|Delay (+ (Variables|Sequence|GetDelayOnEnd) (Variables|Default|GetStoryModeValue)))
  (CallFunction|ToggleHide true))

(fn ConstructionScript
  (|CallParentFunction))
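; Trigger volume that respawns the first-person player at the level's first found RespawnPoint when anything overlaps its box.
; It locks move and look input, matches the point's rotation and location, stops movement, and restores both ability values after re-running ability setup.
; It also resets the first AbilityController found, if any, then re-enables input after a short delay.
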(event OnComponentBeginOverlap(Box)
  (params (OtherActor :type Actor%20Object%20Reference) (OtherComp :type Primitive%20Component%20Object%20Reference) (OtherBodyIndex :type Integer) (bFromSweep :type Boolean) (SweepResult :type Hit%20Result%20Structure%20%28by%20ref%29))
  (bind _returnvalue (Game|GetPlayerController 0))
  (Input|SetIgnoreMoveInput (Game|GetPlayerController 0) true)
  (Input|SetIgnoreLookInput (Game|GetPlayerController 0) true)
  (bind _outactors (Actor|GetAllActorsOfClass "/Game/MyContent/Blueprints/RespawnPoint.RespawnPoint_C"))
  (Pawn|SetControlRotation (Game|GetPlayerController 0) (Transformation|GetWorldRotation (Variables|/Game/MyContent/Blueprints/RespawnPoint.RespawnPoint_C|GetRoot (Utilities|Array|Get(acopy) _outactors))))
  (bind _asmy_fpcharacter (Utilities|Casting|CastToMyFPCharacter (Game|GetPlayerCharacter 0)))
  (Class|NavMovementComponent|StopActiveMovement (Variables|/Script/Engine.Character|GetCharacterMovement _asmy_fpcharacter))
  (Default|SetupAbilities _asmy_fpcharacter "NewEnumerator0")
  (Variables|/Game/MyContent/Blueprints/MyFPCharacter.MyFPCharacter_C|SetLeftAbilityValue _asmy_fpcharacter 100)
  (Variables|/Game/MyContent/Blueprints/MyFPCharacter.MyFPCharacter_C|SetRightAbilityValue _asmy_fpcharacter 100)
  (Transformation|SetActorLocation (Pawn|GetControlledPawn (Game|GetPlayerController 0)) (Transformation|GetWorldLocation (Variables|/Game/MyContent/Blueprints/RespawnPoint.RespawnPoint_C|GetRoot (Utilities|Array|Get(acopy) _outactors))) false false)
  (bind _outactors_2 (Actor|GetAllActorsOfClass "/Game/MyContent/Blueprints/AbilityController.AbilityController_C"))
  (if (> (Utilities|Array|Length _outactors_2) 0)
    (Default|ResetEvent (Utilities|Array|Get(acopy) _outactors_2)))
  (Utilities|FlowControl|Delay 0.5)
  (Input|ResetIgnoreLookInput _returnvalue)
  (Input|ResetIgnoreMoveInput _returnvalue))

(fn ConstructionScript)
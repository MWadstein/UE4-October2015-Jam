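; Trigger volume that plays a one-time intro conversation between Mathew and Michelle when the player enters a red, blue or green room area.
; It reads SaveSlot1 to mute dialogue if sounds are off and to count completed rooms, which picks the lead-in and follow-up lines around the area's intro.
; Timed delays sequence the lines while the player's walk speed is changed, then speed is restored and an optional linked door animates.
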(event OnComponentBeginOverlap(Box)
  (params (OtherActor :type Actor%20Object%20Reference) (OtherComp :type Primitive%20Component%20Object%20Reference) (OtherBodyIndex :type Integer) (bFromSweep :type Boolean) (SweepResult :type Hit%20Result%20Structure%20%28by%20ref%29))
  (if (not (Variables|Default|GetHasTriggered))
    (Variables|Default|SetHasTriggered true)
    (if (Utilities|DoesObjectImplementInterface OtherActor "/Game/MyContent/Blueprints/Interfaces/Player.Player_C")
      (bind _returnvalue (SaveGame|LoadGamefromSlot "SaveSlot1"))
      (bind _asmy_save_game (Utilities|Casting|CastToMySaveGame _returnvalue))
      (Variables|Default|SetSaveInstance _asmy_save_game)
      (if (Variables|/Game/MyContent/Blueprints/Base/MySaveGame.MySaveGame_C|GetSounds (Variables|Default|GetSaveInstance))
        _
        (else
          (Variables|Default|SetVolume 0.0)))
      (Utilities|FlowControl|Sequence ; how many rooms?
        (:then_0
          ;[1 1 1] How many rooms completed?
          (if (Variables|/Game/MyContent/Blueprints/Base/MySaveGame.MySaveGame_C|GetSavedRed (Variables|Default|GetSaveInstance))
            (Variables|Default|SetRoomsCompleted (+ (Variables|Default|GetRoomsCompleted) 1))))
        (:then_1
          (if (Variables|/Game/MyContent/Blueprints/Base/MySaveGame.MySaveGame_C|GetSavedBlue (Variables|Default|GetSaveInstance))
            (Variables|Default|SetRoomsCompleted (+ (Variables|Default|GetRoomsCompleted) 1))))
        (:then_2
          (if (Variables|/Game/MyContent/Blueprints/Base/MySaveGame.MySaveGame_C|GetSavedGreen (Variables|Default|GetSaveInstance))
            (Variables|Default|SetRoomsCompleted (+ (Variables|Default|GetRoomsCompleted) 1))))
        (:then_3
          (CallFunction|ToggleWalkSpeed true) ; make them walk
          ;[1 1 1] Pre Intro voice
          (switch int (Variables|Default|GetRoomsCompleted)
            (:Default
              (Class|GameplayStatics|PlayDialogueatLocation "/Game/MyContent/Audio/Mathew/DW_mathew-MichelleHeresWhatYouNeed.DW_mathew-MichelleHeresWhatYouNeed" (Variables|Default|GetDC_Mathew) (Transformation|GetWorldLocation (Variables|Default|GetRoot)) "0, 0, 0" (Variables|Default|GetVolume) :!label _label)
              (Utilities|FlowControl|Delay 2.5))
            (:0
              (Class|GameplayStatics|PlayDialogueatLocation "/Game/MyContent/Audio/Mathew/DW_mathew-OkHunny.DW_mathew-OkHunny" (Variables|Default|GetDC_Mathew) (Transformation|GetWorldLocation (Variables|Default|GetRoot)) "0, 0, 0" (Variables|Default|GetVolume))
              (Utilities|FlowControl|Delay 1.2))
            (:1
              (Class|GameplayStatics|PlayDialogueatLocation "/Game/MyContent/Audio/Mathew/DW_mathew-OkMichelle.DW_mathew-OkMichelle" (Variables|Default|GetDC_Mathew) (Transformation|GetWorldLocation (Variables|Default|GetRoot)) "0, 0, 0" (Variables|Default|GetVolume))
              (Utilities|FlowControl|Delay 1.5))
            (:2
              (goto _label)))
          ;[1 1 1] Room Intro
          (switch Utilities|FlowControl|Switch|SwitchonAreas (Variables|Default|GetArea)
            (:NewEnumerator1
              (Class|GameplayStatics|PlayDialogueatLocation "/Game/MyContent/Audio/Mathew/DW_mathew-RedRoomIntro.DW_mathew-RedRoomIntro" (Variables|Default|GetDC_Mathew) (Transformation|GetWorldLocation (Variables|Default|GetRoot)) "0, 0, 0" (Variables|Default|GetVolume))
              (Utilities|FlowControl|Delay 1e+01))
            (:NewEnumerator2
              (Class|GameplayStatics|PlayDialogueatLocation "/Game/MyContent/Audio/Mathew/DW_mathew-BlueRoomIntro.DW_mathew-BlueRoomIntro" (Variables|Default|GetDC_Mathew) (Transformation|GetWorldLocation (Variables|Default|GetRoot)) "0, 0, 0" (Variables|Default|GetVolume))
              (Utilities|FlowControl|Delay 9.5))
            (:NewEnumerator3
              (Class|GameplayStatics|PlayDialogueatLocation "/Game/MyContent/Audio/Mathew/DW_mathew-GreenRoomIntro.DW_mathew-GreenRoomIntro" (Variables|Default|GetDC_Mathew) (Transformation|GetWorldLocation (Variables|Default|GetRoot)) "0, 0, 0" (Variables|Default|GetVolume))
              (Utilities|FlowControl|Delay 7.5)))
          ;[1 1 1] Post Intro Voice 1
          (switch int (Variables|Default|GetRoomsCompleted)
            (:Default
              (Class|GameplayStatics|PlayDialogueatLocation "/Game/MyContent/Audio/Michelle/DW_michelle-ICantDoThis.DW_michelle-ICantDoThis" (Variables|Default|GetDC_Michelle) (Transformation|GetWorldLocation (Variables|Default|GetRoot)) "0, 0, 0" (Variables|Default|GetVolume) :!label _label_2)
              (Utilities|FlowControl|Delay 2.4))
            (:0
              (Class|GameplayStatics|PlayDialogueatLocation "/Game/MyContent/Audio/Michelle/DW_michelle-OkICanDoThis.DW_michelle-OkICanDoThis" (Variables|Default|GetDC_Michelle) (Transformation|GetWorldLocation (Variables|Default|GetRoot)) "0, 0, 0" (Variables|Default|GetVolume))
              (Utilities|FlowControl|Delay 2.5))
            (:1
              (Class|GameplayStatics|PlayDialogueatLocation "/Game/MyContent/Audio/Michelle/DW_michelle-IDontKnow.DW_michelle-IDontKnow" (Variables|Default|GetDC_Michelle) (Transformation|GetWorldLocation (Variables|Default|GetRoot)) "0, 0, 0" (Variables|Default|GetVolume))
              (Utilities|FlowControl|Delay 1.8))
            (:2
              (goto _label_2)))
          ;[1 1 1] Post Intro Voice 2
          (switch int (Variables|Default|GetRoomsCompleted)
            (:Default
              (Class|GameplayStatics|PlayDialogueatLocation "/Game/MyContent/Audio/Mathew/DW_mathew-1KidLet.DW_mathew-1KidLet" (Variables|Default|GetDC_Mathew) (Transformation|GetWorldLocation (Variables|Default|GetRoot)) "0, 0, 0" (Variables|Default|GetVolume) :!label _label_3)
              (Utilities|FlowControl|Delay 2.5))
            (:0
              (Class|GameplayStatics|PlayDialogueatLocation "/Game/MyContent/Audio/Mathew/DW_mathew-3KidsLeft.DW_mathew-3KidsLeft" (Variables|Default|GetDC_Mathew) (Transformation|GetWorldLocation (Variables|Default|GetRoot)) "0, 0, 0" (Variables|Default|GetVolume))
              (Utilities|FlowControl|Delay 2.5))
            (:1
              (Class|GameplayStatics|PlayDialogueatLocation "/Game/MyContent/Audio/Mathew/DW_mathew-2KidsLeft.DW_mathew-2KidsLeft" (Variables|Default|GetDC_Mathew) (Transformation|GetWorldLocation (Variables|Default|GetRoot)) "0, 0, 0" (Variables|Default|GetVolume))
              (Utilities|FlowControl|Delay 2.5))
            (:2
              (goto _label_3)))
          (CallFunction|ToggleWalkSpeed false) ; normal speed
          (if (Variables|Default|GetIsTriggeringDoor)
            (Default|AnimateDoor (Variables|Default|GetDoorToTrigger))
            (Variables|Default|SetIsTriggeringDoor false)))))))

(fn ConstructionScript)

(fn ToggleWalkSpeed
  (params (IsSlowed :type Boolean))
  (if IsSlowed
    (bind _asmy_fpcharacter (Utilities|Casting|CastToMyFPCharacter (Game|GetPlayerCharacter 0)))
    (Variables|Default|SetMovementComp (Variables|/Script/Engine.Character|GetCharacterMovement _asmy_fpcharacter))
    (Variables|Default|SetOriginalWalkSpeed (Variables|/Script/Engine.CharacterMovementComponent|GetMaxWalkSpeed (Variables|/Script/Engine.Character|GetCharacterMovement _asmy_fpcharacter)))
    (Variables|/Script/Engine.CharacterMovementComponent|SetMaxWalkSpeed (Variables|Default|GetMovementComp) (Variables|Default|GetNewWalkSpeed))
    (else
      (Variables|/Script/Engine.CharacterMovementComponent|SetMaxWalkSpeed (Variables|Default|GetMovementComp) (Variables|Default|GetOriginalWalkSpeed)))))
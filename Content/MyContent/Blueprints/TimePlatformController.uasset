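; Controller that cycles groups of timed platforms through a looping sequence of start and end steps.
; It begins on BeginPlay with AutoStart, otherwise on Box overlap, setting two looping timers from StartDelay and EndDelay.
; StartSequence starts the current step's PlatformsStart; EndSequence ends its PlatformsEnd, then advances and wraps the shared index.
; RunSequence combines both phases but is not called within this Blueprint.
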(event OnComponentBeginOverlap(Box)
  (params (OtherActor :type Actor%20Object%20Reference) (OtherComp :type Primitive%20Component%20Object%20Reference) (OtherBodyIndex :type Integer) (bFromSweep :type Boolean) (SweepResult :type Hit%20Result%20Structure%20%28by%20ref%29))
  (if (not (Variables|Default|GetAutoStart))
    (Utilities|Time|SetTimerbyFunctionName 0 "StartSequence" (Variables|Default|GetStartDelay) true)
    (Utilities|Time|SetTimerbyFunctionName 0 "EndSequence" (Variables|Default|GetEndDelay) true)))

(event EventBeginPlay
  (if (Variables|Default|GetAutoStart)
    (Utilities|Time|SetTimerbyFunctionName 0 "StartSequence" (Variables|Default|GetStartDelay) true)
    (Utilities|Time|SetTimerbyFunctionName 0 "EndSequence" (Variables|Default|GetEndDelay) true)))

(fn ConstructionScript)

(fn StartSequence
  (for _array_element (Variables|/Game/MyContent/Blueprints/ArrayOfPlatforms.ArrayOfPlatforms_C|GetPlatformsStart (Utilities|Array|Get(acopy) (Variables|Default|GetPlatformSequence) (Variables|Default|GetCurrentLoopIndex)))
    (Default|StartSequence _array_element)))

(fn EndSequence
  (Utilities|FlowControl|Sequence
    (:then_0
      (for _array_element (Variables|/Game/MyContent/Blueprints/ArrayOfPlatforms.ArrayOfPlatforms_C|GetPlatformsEnd (Utilities|Array|Get(acopy) (Variables|Default|GetPlatformSequence) (Variables|Default|GetCurrentLoopIndex)))
        (Default|EndSequence _array_element)))
    (:then_1
      (Variables|Default|SetCurrentLoopIndex (+ (Variables|Default|GetCurrentLoopIndex) 1))
      (if (== (Variables|Default|GetCurrentLoopIndex) (Utilities|Array|Length (Variables|Default|GetPlatformSequence)))
        (Variables|Default|SetCurrentLoopIndex 0)))))

(fn RunSequence
  (Utilities|FlowControl|Sequence
    (:then_0
      (for _array_element (Variables|/Game/MyContent/Blueprints/ArrayOfPlatforms.ArrayOfPlatforms_C|GetPlatformsStart (Utilities|Array|Get(acopy) (Variables|Default|GetPlatformSequence) (Variables|Default|GetCurrentLoopIndex)))
        (Default|StartSequence _array_element)))
    (:then_1
      (for _array_element_2 (Variables|/Game/MyContent/Blueprints/ArrayOfPlatforms.ArrayOfPlatforms_C|GetPlatformsEnd (Utilities|Array|Get(acopy) (Variables|Default|GetPlatformSequence) (Variables|Default|GetCurrentLoopIndex)))
        (Default|EndSequence _array_element_2)))
    (:then_2
      (Variables|Default|SetCurrentLoopIndex (+ (Variables|Default|GetCurrentLoopIndex) 1))
      (if (== (Variables|Default|GetCurrentLoopIndex) (Utilities|Array|Length (Variables|Default|GetPlatformSequence)))
        (Variables|Default|SetCurrentLoopIndex 0)))))
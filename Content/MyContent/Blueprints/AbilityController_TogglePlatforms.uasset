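; Ability controller that lets the player toggle Left and Right platform groups between hidden and visible when enough power remains.
; Showing a group starts a looping timer that drains that side's power on MyFPCharacter; hiding it starts a recharge timer.
; Running out of power force-hides the group, and a reset event clears both timers and hides all platforms.
; Story mode, read from the save game, scales the drain interval.
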(event EventPlayerUsedAbility
  (params (Ability :type Name) (CurrentPower :type Integer))
  (CallFunction|TogglethePlatforms Ability false CurrentPower))

(event EventBeginPlay
  (CallFunction|SetStoryMode))

(event EventCheckStoryMode
  (CallFunction|SetStoryMode))

(event EventAbilityOutOfPower
  (params (Ability :type Name))
  (CallFunction|TogglethePlatforms Ability true))

(event EventClearTimer
  (params (Ability :type Name))
  (CallFunction|ClearActiveTimer Ability))

(event EventResetEvent
  (CallFunction|ClearActiveTimer "Left")
  (CallFunction|ClearActiveTimer "Right")
  (CallFunction|ResetPlatforms))

(fn ConstructionScript
  (|CallParentFunction))

(fn TogglethePlatforms
  (params (Ability :type Name) (ShutItOff :type Boolean) (AbilityPower :type Integer))
  (bind _output_get (LocalVariables|SetWhichAbility Ability))
  (LocalVariables|SetShutOff ShutItOff)
  (LocalVariables|SetAbilityValue AbilityPower)
  (if (Utilities|Name|Equal(Name) _output_get "Left") ; Left or Right
    (if (LocalVariables|GetShutOff)
      (LocalVariables|SetIsHidden true)
      (for _array_element (Variables|Platforms|GetLeftPlatforms) :!label _label
        (Default|ToggleHintMaterial _array_element)
        (Default|ToggleHide _array_element (LocalVariables|GetIsHidden))
        (Variables|Default|SetLeftVisibility (not (LocalVariables|GetIsHidden)))
        (if (LocalVariables|GetShutOff)
          (CallFunction|ClearActiveTimer "Left")
          (bind _returnvalue (Utilities|Time|SetTimerbyFunctionName 0 "IncreaseLeftPower" (Variables|TimeValues|GetLeftRechargeTick) true))
          (Variables|Default|SetLeftTimer _returnvalue)
          (else
            (CallFunction|LeftAbilityUsed))))
      (elif (<= (Math|Integer|Absolute(Integer) (Variables|TimeValues|GetLeftDischargeRate)) (LocalVariables|GetAbilityValue)) ; enough power?
        (LocalVariables|SetIsHidden (Variables|Default|GetLeftVisibility))
        (goto _label)))
    (elif (LocalVariables|GetShutOff)
      (LocalVariables|SetIsHidden true)
      (for _array_element_2 (Variables|Platforms|GetRightPlatforms) :!label _label_2
        (Default|ToggleHintMaterial _array_element_2)
        (Default|ToggleHide _array_element_2 (LocalVariables|GetIsHidden))
        (Variables|Default|SetRightVisibility (not (LocalVariables|GetIsHidden)))
        (if (LocalVariables|GetShutOff)
          (CallFunction|ClearActiveTimer "Right")
          (bind _returnvalue_2 (Utilities|Time|SetTimerbyFunctionName 0 "IncreaseRightPower" (Variables|TimeValues|GetRightRechargeTick) true))
          (Variables|Default|SetRightTimer _returnvalue_2)
          (else
            (CallFunction|RightAbilityUsed))))
      (elif (<= (Math|Integer|Absolute(Integer) (Variables|TimeValues|GetRightDischargeRate)) (LocalVariables|GetAbilityValue)) ; enough power?
        (LocalVariables|SetIsHidden (Variables|Default|GetRightVisibility))
        (goto _label_2)))))

(fn DecreaseLeftPower
  (bind _asmy_fpcharacter (Utilities|Casting|CastToMyFPCharacter (Game|GetPlayerCharacter 0)))
  (Default|ChangeAbilityValue _asmy_fpcharacter (Variables|TimeValues|GetLeftDischargeRate) "Left"))

(fn DecreaseRightPower
  (bind _asmy_fpcharacter (Utilities|Casting|CastToMyFPCharacter (Game|GetPlayerCharacter 0)))
  (Default|ChangeAbilityValue _asmy_fpcharacter (Variables|TimeValues|GetRightDischargeRate) "Right"))

(fn LeftAbilityUsed
  (if (Variables|Default|GetLeftVisibility)
    (Class|KismetSystemLibrary|ClearTimerHandle (Variables|Default|GetLeftTimer))
    (bind _returnvalue (Utilities|Time|SetTimerbyFunctionName 0 "DecreaseLeftPower" (* (Variables|TimeValues|GetLeftDischargeTick) (Variables|Default|GetStoryModeAmount)) true))
    (Variables|Default|SetLeftTimer _returnvalue)
    (else
      (Class|KismetSystemLibrary|ClearTimerHandle (Variables|Default|GetLeftTimer))
      (bind _returnvalue_2 (Utilities|Time|SetTimerbyFunctionName 0 "IncreaseLeftPower" (Variables|TimeValues|GetLeftRechargeTick) true))
      (Variables|Default|SetLeftTimer _returnvalue_2))))

(fn RightAbilityUsed
  (if (Variables|Default|GetRightVisibility)
    (Class|KismetSystemLibrary|ClearTimerHandle (Variables|Default|GetRightTimer))
    (bind _returnvalue (Utilities|Time|SetTimerbyFunctionName 0 "DecreaseRightPower" (* (Variables|TimeValues|GetRightDischageTick) (Variables|Default|GetStoryModeAmount)) true))
    (Variables|Default|SetRightTimer _returnvalue)
    (else
      (Class|KismetSystemLibrary|ClearTimerHandle (Variables|Default|GetRightTimer))
      (bind _returnvalue_2 (Utilities|Time|SetTimerbyFunctionName 0 "IncreaseRightPower" (Variables|TimeValues|GetRightRechargeTick) true))
      (Variables|Default|SetRightTimer _returnvalue_2))))

(fn IncreaseRightPower
  (bind _asmy_fpcharacter (Utilities|Casting|CastToMyFPCharacter (Game|GetPlayerCharacter 0)))
  (Default|ChangeAbilityValue _asmy_fpcharacter (Variables|TimeValues|GetRightRechargeRate) "Right"))

(fn IncreaseLeftPower
  (bind _asmy_fpcharacter (Utilities|Casting|CastToMyFPCharacter (Game|GetPlayerCharacter 0)))
  (Default|ChangeAbilityValue _asmy_fpcharacter (Variables|TimeValues|GetLeftRechargeRate) "Left"))

(fn ClearActiveTimer
  (params (Ability :type Name))
  (if (Utilities|Name|Equal(Name) Ability "Left")
    (Class|KismetSystemLibrary|ClearTimerHandle (Variables|Default|GetLeftTimer))
    (else
      (Class|KismetSystemLibrary|ClearTimerHandle (Variables|Default|GetRightTimer)))))

(fn ResetPlatforms
  (Utilities|FlowControl|Sequence
    (:then_0
      (for _array_element (Variables|Platforms|GetLeftPlatforms)
        (Default|ToggleHide _array_element true)
        (Variables|Default|SetLeftVisibility false)))
    (:then_1
      (for _array_element_2 (Variables|Platforms|GetRightPlatforms)
        (Default|ToggleHide _array_element_2 true)
        (Variables|Default|SetRightVisibility false)))))

(fn SetStoryMode
  (bind _returnvalue (SaveGame|LoadGamefromSlot "SaveSlot1"))
  (bind _asmy_save_game (Utilities|Casting|CastToMySaveGame _returnvalue))
  (if (Variables|/Game/MyContent/Blueprints/Base/MySaveGame.MySaveGame_C|GetStoryMode _asmy_save_game)
    (Variables|Default|SetStoryModeAmount (Variables|Default|GetStoryModeAdjust))
    (else
      (Variables|Default|SetStoryModeAmount 1.0))))
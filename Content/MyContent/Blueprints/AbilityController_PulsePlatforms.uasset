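; Ability controller that spends the player's Left ability power to pulse a set of platforms in a staggered sequence.
; Each platform's start is delayed by its array index, and its on-time is extended when the save game has Story Mode enabled.
; Using the ability starts a looping timer that recharges power on the player character.
; Reset events clear that timer and reset every platform.
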(event EventCheckStoryMode
  (CallFunction|SetStoryMode))

(event EventBeginPlay
  (CallFunction|SetStoryMode))

(event EventPlayerUsedAbility
  (params (Ability :type Name) (CurrentPower :type Integer))
  (CallFunction|PulsePlatforms CurrentPower Ability))

(event EventResetEvent
  (CallFunction|ClearActiveTimer "Left")
  (CallFunction|ResetPlatforms))

(event EventAbilityOutOfPower
  (params (Ability :type Name :default "None")))

(event EventClearTimer
  (params (Ability :type Name))
  (CallFunction|ClearActiveTimer Ability))

(fn ConstructionScript
  (|CallParentFunction))

(fn PulsePlatforms
  (params (AbilityPower :type Integer) (Ability :type Name))
  (LocalVariables|SetAbilityValue AbilityPower)
  (if (Utilities|Name|Equal(Name) Ability "Left") ; Left or Right
    (if (<= (Math|Integer|Absolute(Integer) (Variables|Default|GetPulseCost)) (LocalVariables|GetAbilityValue)) ; enough power?
      (for (_array_element _array_index) (Variables|Default|GetPlatforms)
        (Default|Pulse _array_element (* _array_index (Variables|Default|GetDelayBetweenPulses)) (+ (Variables|Default|GetPulseOnTime) (Variables|Default|GetStoryModeAmount))))
      (bind _asmy_fpcharacter (Utilities|Casting|CastToMyFPCharacter (Game|GetPlayerCharacter 0)))
      (Default|ChangeAbilityValue _asmy_fpcharacter (Variables|Default|GetPulseCost) "Left")
      (CallFunction|LeftAbilityUsed))))

(fn ClearActiveTimer
  (params (Ability :type Name))
  (if (Utilities|Name|Equal(Name) Ability "Left")
    (Class|KismetSystemLibrary|ClearTimerHandle (Variables|Default|GetLeftTimer))))

(fn IncreaseLeftPower
  (bind _asmy_fpcharacter (Utilities|Casting|CastToMyFPCharacter (Game|GetPlayerCharacter 0)))
  (Default|ChangeAbilityValue _asmy_fpcharacter (Variables|Default|GetRechargeAmount) "Left" (Variables|Default|GetPulseCost)))

(fn LeftAbilityUsed
  (Class|KismetSystemLibrary|ClearTimerHandle (Variables|Default|GetLeftTimer))
  (bind _returnvalue (Utilities|Time|SetTimerbyFunctionName 0 "IncreaseLeftPower" (Variables|Default|GetRechargeTick) true))
  (Variables|Default|SetLeftTimer _returnvalue))

(fn SetStoryMode
  (bind _returnvalue (SaveGame|LoadGamefromSlot "SaveSlot1"))
  (bind _asmy_save_game (Utilities|Casting|CastToMySaveGame _returnvalue))
  (if (Variables|/Game/MyContent/Blueprints/Base/MySaveGame.MySaveGame_C|GetStoryMode _asmy_save_game)
    (Variables|Default|SetStoryModeAmount (Variables|Default|GetStoryModeAdjust))
    (else
      (Variables|Default|SetStoryModeAmount 0.0))))

(fn ResetPlatforms
  (for _array_element (Variables|Default|GetPlatforms)
    (Default|ResetPlatform _array_element)))
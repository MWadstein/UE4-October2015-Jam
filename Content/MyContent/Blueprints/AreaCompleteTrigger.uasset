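; Trigger actor that completes an area and sends the player back to the main room.
; Any overlap with its box destroys the first RespawnPoint found and streams in MainRoom.
; It then respawns the MyFPCharacter player at a spawn point, reports AreaCompleted to that character and unloads the CurrentRoom level.
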(event OnComponentBeginOverlap(Box)
  (params (OtherActor :type Actor%20Object%20Reference) (OtherComp :type Primitive%20Component%20Object%20Reference) (OtherBodyIndex :type Integer) (bFromSweep :type Boolean) (SweepResult :type Hit%20Result%20Structure%20%28by%20ref%29))
  (bind _outactors (Actor|GetAllActorsOfClass "/Game/MyContent/Blueprints/RespawnPoint.RespawnPoint_C"))
  (Actor|DestroyActor (Utilities|Array|Get(acopy) _outactors))
  (Game|LoadStreamLevel(byName) "MainRoom" true)
  (bind _asmy_fpcharacter (Utilities|Casting|CastToMyFPCharacter (Game|GetPlayerCharacter 0)))
  (Default|RespawnatSpawnPoint _asmy_fpcharacter false)
  (Default|PlayerCompletedArea _asmy_fpcharacter (Variables|Default|GetAreaCompleted))
  (Game|UnloadStreamLevel(byName) (Variables|Default|GetCurrentRoom)))

(fn ConstructionScript)
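; A box trigger actor that manages level streaming and related progression events when anything begins overlapping it.
; Flags select each step: load, unload or show a named streaming level, animate a linked door once, or save.
; Saving loads or creates the MySaveGame in SaveSlot1 and records the map name.
; After a short delay, it can also apply a new ability set to the player character.
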(event OnComponentBeginOverlap(Box)
  (params (OtherActor :type Actor%20Object%20Reference) (OtherComp :type Primitive%20Component%20Object%20Reference) (OtherBodyIndex :type Integer) (bFromSweep :type Boolean) (SweepResult :type Hit%20Result%20Structure%20%28by%20ref%29))
  (bind _visiblelevelname (Variables|Default|GetVisibleLevelName))
  (bind _returnvalue (Class|GameplayStatics|GetStreamingLevel _visiblelevelname))
  (Utilities|FlowControl|Sequence
    (:then_0
      (if (Variables|Default|GetIsLoading)
        (if (not (Class|LevelStreaming|IsLevelLoaded (Class|GameplayStatics|GetStreamingLevel (Variables|Default|GetLoadLevelName))))
          (Game|LoadStreamLevel(byName) (Variables|Default|GetLoadLevelName) (Variables|Default|GetIsMakingVisible)))))
    (:then_1
      (if (Variables|Default|GetIsUnloading)
        (if (Class|LevelStreaming|IsLevelLoaded (Class|GameplayStatics|GetStreamingLevel (Variables|Default|GetUnloadLevelName)))
          (Game|UnloadStreamLevel(byName) (Variables|Default|GetUnloadLevelName)))))
    (:then_2
      (if (Variables|Default|GetIsMakingVisible)
        (if (not (Class|LevelStreaming|IsLevelVisible _returnvalue))
          (Variables|/Script/Engine.LevelStreaming|SetbShouldBeVisible _returnvalue true))))
    (:then_3
      (if (Variables|Default|GetIsTriggeringDoor)
        (Default|AnimateDoor (Variables|Default|GetDoorToTrigger))
        (Variables|Default|SetIsTriggeringDoor false)))
    (:then_4
      (if (Variables|Default|GetSaveGame)
        (bind _returnvalue_2 (SaveGame|LoadGamefromSlot "SaveSlot1"))
        (bind _asmy_save_game (Utilities|Casting|CastToMySaveGame _returnvalue_2)
          (:then
            (Variables|Default|SetSaveInstance _asmy_save_game))
          (:CastFailed
            (bind _returnvalue_3 (SaveGame|CreateSaveGameObject "/Game/MyContent/Blueprints/MySaveGame.MySaveGame_C"))
            (bind _asmy_save_game_2 (Utilities|Casting|CastToMySaveGame _returnvalue_3))
            (Variables|Default|SetSaveInstance _asmy_save_game_2)))
        (Variables|/Game/MyContent/Blueprints/MySaveGame.MySaveGame_C|SetCurrentMap (Variables|Default|GetSaveInstance) (Variables|Default|GetMapNameForSave))
        (Variables|/Game/MyContent/Blueprints/MySaveGame.MySaveGame_C|SetSavedBlue (Variables|Default|GetSaveInstance) (Variables|/Game/MyContent/Blueprints/MySaveGame.MySaveGame_C|GetSavedBlue (Variables|Default|GetSaveInstance)))
        (Variables|/Game/MyContent/Blueprints/MySaveGame.MySaveGame_C|SetSavedGreen (Variables|Default|GetSaveInstance) (Variables|/Game/MyContent/Blueprints/MySaveGame.MySaveGame_C|GetSavedGreen (Variables|Default|GetSaveInstance)))
        (Variables|/Game/MyContent/Blueprints/MySaveGame.MySaveGame_C|SetSavedRed (Variables|Default|GetSaveInstance) (Variables|/Game/MyContent/Blueprints/MySaveGame.MySaveGame_C|GetSavedRed (Variables|Default|GetSaveInstance)))
        (SaveGame|SaveGametoSlot (Variables|Default|GetSaveInstance) "SaveSlot1")))
    (:then_5
      (Utilities|FlowControl|Delay 0.5)
      (if (Variables|Default|GetToggleAbilities)
        (bind _asmy_fpcharacter (Utilities|Casting|CastToMyFPCharacter (Game|GetPlayerCharacter 0)))
        (Default|SetupAbilities _asmy_fpcharacter (Variables|Default|GetNewAbilities))))))

(event EventBeginPlay)

(fn ConstructionScript)
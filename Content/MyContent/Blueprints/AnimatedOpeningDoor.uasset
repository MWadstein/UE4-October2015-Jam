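; AnimatedOpeningDoor is a door Blueprint that opens by sinking into the ground.
; BeginPlay caches the root's world location as the starting position.
; The AnimateDoor event plays a timeline that lerps the root 300 units straight down from that position, without sweep, and destroys the actor on finish when DestroyWhenDone is set.
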(event Custom|AnimateDoor
  (bind _startingposition (Variables|Default|GetStartingPosition))
  (bind _lerp_0_1 (Timeline|Timeline_0 PlayFromStart)
    (:Update
      (Transformation|SetWorldLocation (Variables|Default|GetRoot) (Math|Vector|Lerp(Vector) (Math|Vector|MakeVector (.x _startingposition) (.y _startingposition) (.z _startingposition)) (Math|Vector|MakeVector (.x _startingposition) (.y _startingposition) (- (.z _startingposition) 3e+02)) _lerp_0_1) false false))
    (:Finished
      (if (Variables|Default|GetDestroyWhenDone)
        (Actor|DestroyActor)))))

(event EventBeginPlay
  (Variables|Default|SetStartingPosition (Transformation|GetWorldLocation (Variables|Default|GetRoot))))

(fn ConstructionScript)